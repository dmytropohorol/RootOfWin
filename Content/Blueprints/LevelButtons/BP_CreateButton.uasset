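; BP_CreateButton is a floor button that BP_ROWCharacter or BP_Cube presses to spawn a configured list of actors at preset transforms.
; Box1 overlaps move Cylinder1 and play on/off sounds, with DoOnce limiting spawning to the first press.
; CheckForActors scans for other occupants, preventing repeat presses and early release.
; After a short exit delay, release starts a one-second lockout, then Reset re-presses if still occupied.
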(event OnComponentBeginOverlap(Box1)
  (params (OverlappedComponent :type Primitive%20Component%20Object%20Reference) (OtherActor :type Actor%20Object%20Reference) (OtherComp :type Primitive%20Component%20Object%20Reference) (OtherBodyIndex :type Integer) (bFromSweep :type Boolean) (SweepResult :type Hit%20Result%20Structure%20%28by%20ref%29))
  (if (Variables|Default|GetisTimerEnded?)
    (if (== (Utilities|GetClass OtherActor) "/Game/Blueprints/BP_ROWCharacter.BP_ROWCharacter_C")
      (bind _occupation (CallFunction|CheckforActors OtherActor false :!label _label))
      (if _occupation
        (if (not (Variables|Default|GetisPressed?))
          (Variables|Default|SetOther%20Actor OtherActor :!label _label_2)
          (Variables|Default|SetisPressed? true)
          (Components|MoveComponentTo (Variables|Default|GetCylinder1) "1.000000,1.000000,0.418798" "0, 0, 0" false false 0.2 false)
          (Audio|PlaySoundatLocation "/Game/Audio/SFX/Button_ON.Button_ON" (Transformation|GetActorLocation) "0, 0, 0" 1.0 1.0 0.0 "/Game/Audio/MainSoundAttenuation.MainSoundAttenuation" 0 0 0)
          (Utilities|FlowControl|DoOnce false
            (:Completed
              (for (_array_element _array_index) (Variables|Default|GetActorsToCreate)
                (Game|SpawnActorfromClass _array_element (Utilities|Array|Get(acopy) (Variables|Default|GetActorsTransform) _array_index) "Undefined" 0 0)))))
        (else
          (goto _label_2)))
      (elif (== (Utilities|GetClass OtherActor) "/Game/Blueprints/BP_Cube.BP_Cube_C")
        (goto _label)))))

(event OnComponentEndOverlap(Box1)
  (params (OverlappedComponent :type Primitive%20Component%20Object%20Reference) (OtherActor :type Actor%20Object%20Reference) (OtherComp :type Primitive%20Component%20Object%20Reference) (OtherBodyIndex :type Integer))
  (Utilities|FlowControl|Delay 0.2)
  (if (Variables|Default|GetisTimerEnded?)
    (if (== (Utilities|GetClass OtherActor) "/Game/Blueprints/BP_ROWCharacter.BP_ROWCharacter_C")
      (bind _occupation (CallFunction|CheckforActors 0 true :!label _label))
      (if (not _occupation)
        (Variables|Default|SetisTimerEnded? false)
        (Variables|Default|SetisPressed? false)
        (Components|MoveComponentTo (Variables|Default|GetCylinder1) "1.000000,1.000000,8.670346" "0, 0, 0" false false 0.2 false)
        (Audio|PlaySoundatLocation "/Game/Audio/SFX/Button_OFF.Button_OFF" (Transformation|GetActorLocation) "0, 0, 0" 1.0 1.0 0.0 "/Game/Audio/MainSoundAttenuation.MainSoundAttenuation" 0 0 0)
        (Utilities|FlowControl|Sequence
          (:then_0
            (Utilities|Time|SetTimerbyFunctionName 0 "Reset" 1.0))))
      (elif (== (Utilities|GetClass OtherActor) "/Game/Blueprints/BP_Cube.BP_Cube_C")
        (goto _label)))))

(event Custom|Reset
  (Variables|Default|SetisTimerEnded? true)
  (bind _occupation (CallFunction|CheckforActors (Variables|Default|GetOther%20Actor) true))
  (if _occupation
    (CallFunction|Startoverlap)))

(event Custom|Startoverlap
  (if (Variables|Default|GetisTimerEnded?)
    (if (== (Utilities|GetClass (stale OnComponentBeginOverlap(Box1) OtherActor)) "/Game/Blueprints/BP_ROWCharacter.BP_ROWCharacter_C")
      (bind _occupation (CallFunction|CheckforActors (stale OnComponentBeginOverlap(Box1) OtherActor) false :!label _label))
      (if _occupation
        (if (not (Variables|Default|GetisPressed?))
          (Variables|Default|SetOther%20Actor (stale OnComponentBeginOverlap(Box1) OtherActor) :!label _label_2)
          (Variables|Default|SetisPressed? true)
          (Components|MoveComponentTo (Variables|Default|GetCylinder1) "1.000000,1.000000,0.418798" "0, 0, 0" false false 0.2 false)
          (Audio|PlaySoundatLocation "/Game/Audio/SFX/Button_ON.Button_ON" (Transformation|GetActorLocation) "0, 0, 0" 1.0 1.0 0.0 "/Game/Audio/MainSoundAttenuation.MainSoundAttenuation" 0 0 0)
          (Utilities|FlowControl|DoOnce false
            (:Completed
              (for (_array_element _array_index) (Variables|Default|GetActorsToCreate)
                (Game|SpawnActorfromClass _array_element (Utilities|Array|Get(acopy) (Variables|Default|GetActorsTransform) _array_index) "Undefined" 0 0)))))
        (else
          (goto _label_2)))
      (elif (== (Utilities|GetClass (stale OnComponentBeginOverlap(Box1) OtherActor)) "/Game/Blueprints/BP_Cube.BP_Cube_C")
        (goto _label)))))

(fn ConstructionScript)

(fn CheckforActors
  (params (InputPin :type Object%20Object%20Reference) (CheckForSelf :type Boolean))
  (bind _box1 (Variables|Default|GetBox1))
  (bind _box1_2 (Variables|Default|GetBox1))
  (bind _overlappingactors (Collision|GetOverlappingActors _box1 0 :!class /Script/Engine.PrimitiveComponent))
  (bind _overlappingactors_2 (Collision|GetOverlappingActors _box1_2 0 :!class /Script/Engine.PrimitiveComponent))
  (if CheckForSelf
    (LocalVariables|SetOcupation false)
    (if (> (Utilities|Array|Length _overlappingactors_2) 0)
      (bind _array_element (Utilities|Array|ForEachLoopwithBreak _overlappingactors_2 :!label _label)
        (:LoopBody
          (if (== (Utilities|GetClass _array_element) "/Game/Blueprints/BP_ROWCharacter.BP_ROWCharacter_C")
            (LocalVariables|SetOcupation true)
            (goto _label Break)
            (elif (== (Utilities|GetClass _array_element) "/Game/Blueprints/BP_Cube.BP_Cube_C")
              (LocalVariables|SetOcupation true)
              (goto _label Break))))
        (:Completed
          (return (LocalVariables|GetOcupation))))
      (else
        (return (LocalVariables|GetOcupation))))
    (else
      (LocalVariables|SetOcupation false)
      (if (> (Utilities|Array|Length _overlappingactors) 0)
        (bind _array_element_2 (Utilities|Array|ForEachLoopwithBreak _overlappingactors :!label _label_2)
          (:LoopBody
            (if (== (Utilities|GetClass _array_element_2) "/Game/Blueprints/BP_ROWCharacter.BP_ROWCharacter_C")
              (if (== _array_element_2 InputPin)
                _
                (else
                  (LocalVariables|SetOcupation true)
                  (goto _label_2 Break))))
            (if (== (Utilities|GetClass _array_element_2) "/Game/Blueprints/BP_Cube.BP_Cube_C")
              (if (not (== _array_element_2 InputPin))
                (LocalVariables|SetOcupation true)
                (goto _label_2 Break))))
          (:Completed
            (return (LocalVariables|GetOcupation))))
        (else
          (return (LocalVariables|GetOcupation)))))))