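; Enemy character that chases the player when the main character enters its detection sphere.
; Sphere1's begin overlap issues an AI MoveTo toward player 0 and sets IsSeeingPlayer as the move is issued.
; End overlap checks that flag, calls StopMovementImmediately on the movement component without explicitly aborting the move request, then clears the flag.
; Both transitions print debug strings.
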(event OnComponentBeginOverlap(Sphere1)
  (params (OverlappedComponent :type Primitive%20Component%20Object%20Reference) (OtherActor :type Actor%20Object%20Reference) (OtherComp :type Primitive%20Component%20Object%20Reference) (OtherBodyIndex :type Integer) (bFromSweep :type Boolean) (SweepResult :type Hit%20Result%20Structure%20%28by%20ref%29))
  (Utilities|Casting|CastToMainCharacter OtherActor)
  (AI|AIMoveTo self "0, 0, 0" (Game|GetPlayerCharacter 0) 5.0 false
    (:then
      (Development|PrintString "true")
      (Variables|Default|SetIsSeeingPlayer? true))))

(event OnComponentEndOverlap(Sphere1)
  (params (OverlappedComponent :type Primitive%20Component%20Object%20Reference) (OtherActor :type Actor%20Object%20Reference) (OtherComp :type Primitive%20Component%20Object%20Reference) (OtherBodyIndex :type Integer))
  (if (Variables|Default|GetIsSeeingPlayer?)
    (Utilities|Casting|CastToMainCharacter OtherActor)
    (Components|Movement|StopMovementImmediately (Variables|Character|GetCharacterMovement))
    (Development|PrintString "false")
    (Variables|Default|SetIsSeeingPlayer? false)))

(event Collision|EventActorBeginOverlap
  (params (OtherActor :type Actor%20Object%20Reference)))

(fn ConstructionScript)