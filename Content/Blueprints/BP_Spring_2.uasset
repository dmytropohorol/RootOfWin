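; BP_Spring_2 is a looping spring that slides along the Y axis and launches characters caught in its box.
; On BeginPlay the authority moves the root out, then launches any BP_ROWCharacter overlapping Box1 along +Y.
; Chained MoveComponentTo and Delay nodes then retract it and restart the cycle indefinitely.
; Move targets are offsets from the root's world location, fed in as relative locations.
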(event EventBeginPlay
  (bind _defaultsceneroot (Variables|Default|GetDefaultSceneRoot))
  (Networking|SwitchHasAuthority
    (:Authority
      (Components|MoveComponentTo _defaultsceneroot (+ (Transformation|GetWorldLocation _defaultsceneroot) (Math|Vector|MakeVector 0.0 2.5e+02 0.0)) "0, 0, 0" false false (Variables|Default|GetOverTimeMoveComponent) false :!label _label)
      (for _array_element (Collision|GetOverlappingActors (Variables|Default|GetBox1) "/Game/Blueprints/BP_ROWCharacter.BP_ROWCharacter_C" :!class /Script/Engine.PrimitiveComponent)
        (bind _asbp_rowcharacter (Utilities|Casting|CastToBP_ROWCharacter _array_element))
        (Character|LaunchCharacter _asbp_rowcharacter "0.000000,500.000000,0.000000" false false)
        (Utilities|FlowControl|Delay 0.2)
        (Components|MoveComponentTo _defaultsceneroot (+ (Transformation|GetWorldLocation _defaultsceneroot) (Math|Vector|MakeVector 0.0 -2.5e+02 0.0)) "0, 0, 0" false false 2.0 false)
        (Utilities|FlowControl|Delay 1.0)
        (goto _label))
      (Utilities|FlowControl|Delay 0.2)
      (Components|MoveComponentTo _defaultsceneroot (+ (Transformation|GetWorldLocation _defaultsceneroot) (Math|Vector|MakeVector 0.0 -2.5e+02 0.0)) "0, 0, 0" false false 2.0 false)
      (Utilities|FlowControl|Delay 1.0)
      (goto _label))))

(fn ConstructionScript)