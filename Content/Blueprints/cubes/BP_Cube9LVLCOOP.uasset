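; BP_Cube9LVLCOOP is a physics cube, apparently for co-op level 9, that respawns itself when destroyed.
; On spawn it plays a throw or appearance sound depending on ConditionToDrop.
; Hits play an impact sound with a speed-mapped Power parameter, throttled by a randomly reset DoOnce.
; Death, skipped while ConditionToGrab is set, disables physics, triggers an effect, hides the mesh, spawns a replacement and destroys itself.
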(event OnComponentHit(StaticMeshComponent)
  (params (HitComponent :type Primitive%20Component%20Object%20Reference) (OtherActor :type Actor%20Object%20Reference) (OtherComp :type Primitive%20Component%20Object%20Reference) (NormalImpulse :type Vector :default "0, 0, 0") (Hit :type Hit%20Result%20Structure%20%28by%20ref%29))
  (Utilities|FlowControl|Sequence
    (:then_0
      (Utilities|FlowControl|DoOnce false :!label _label
        (:Completed
          (bind _returnvalue (Audio|SpawnSoundatLocation "/Game/Audio/Cube/DropCube_SoundCue.DropCube_SoundCue" (.Location (Collision|BreakHitResult Hit)) "0, 0, 0" 1.0 1.0 0.0 "/Game/Audio/MainSoundAttenuation.MainSoundAttenuation" 0))
          (Effects|Components|ParticleSystem|SetIntParameter _returnvalue "Power" (Math|Float|Truncate (Math|Float|MapRangeClamped (Math|Vector|VectorLength (Transformation|GetVelocity)) 1e+03 4e+01 0.0 4.0))))))
    (:then_1
      (Utilities|FlowControl|Delay (Math|Random|RandomFloatinRange 0.1 0.2))
      (goto _label Reset))))

(event Custom|Death
  (bind _staticmeshcomponent (Variables|Debug|GetStaticMeshComponent))
  (if (not (Variables|Default|GetConditionToGrab))
    (Components|Activation|Activate (Variables|Default|GetDym123123_2) true)
    (Physics|SetSimulatePhysics _staticmeshcomponent false)
    (Collision|SetCollisionEnabled _staticmeshcomponent "NoCollision")
    (Audio|PlaySoundatLocation "/Game/Audio/SFX/Cube_Disappear.Cube_Disappear" (Transformation|GetActorLocation) "0, 0, 0" 1.0 1.0 0.0 "/Game/Audio/MainSoundAttenuation.MainSoundAttenuation" 0 0 0)
    (Components|Activation|Activate (Variables|Default|GetDym123123_2) false)
    (Utilities|FlowControl|Delay 0.55)
    (Development|SetHiddeninGame (Variables|Debug|GetStaticMeshComponent) true false)
    (Utilities|FlowControl|Delay 0.5)
    (Game|SpawnActorfromClass "BP_Cube9LVLCOOP_C" (Math|Transform|MakeTransform (Variables|Default|GetSpawn%20Transform%20Location) "0, 0, 0" "1.000000,1.000000,1.000000") "Undefined" 0 false false 0)
    (Actor|DestroyActor)))

(event EventBeginPlay
  (bind _returnvalue (Transformation|GetActorLocation))
  (if (Variables|Default|GetConditionToDrop)
    (Audio|PlaySoundatLocation "/Game/Audio/Cube/Cube_Throw.Cube_Throw" _returnvalue "0, 0, 0" 1.0 1.0 0.0 "/Game/Audio/MainSoundAttenuation.MainSoundAttenuation" 0 0 0)
    (else
      (Audio|PlaySoundatLocation "/Game/Audio/Cube/CUBE_APPEARANCE.CUBE_APPEARANCE" _returnvalue "0, 0, 0" 1.0 1.0 0.0 "/Game/Audio/MainSoundAttenuation.MainSoundAttenuation" 0 0 0))))

(fn ConstructionScript)