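; BP_COOPTeleportator is a trigger actor that sends a player into the co-op lobby.
; The first BP_ROWCharacter to overlap its box fires a DoOnce that calls TeleportCOOP, then after a short delay calls Tplevel to open COOP_Lobby as a listen server.
; The construction script parses a Level number from the current map name, special-casing "10_2" as 10, though the event graph does not use it.
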(event OnComponentBeginOverlap(Box)
  (params (OverlappedComponent :type Primitive%20Component%20Object%20Reference) (OtherActor :type Actor%20Object%20Reference) (OtherComp :type Primitive%20Component%20Object%20Reference) (OtherBodyIndex :type Integer) (bFromSweep :type Boolean) (SweepResult :type Hit%20Result%20Structure%20%28by%20ref%29))
  (bind _asbp_rowcharacter (Utilities|Casting|CastToBP_ROWCharacter OtherActor))
  (Utilities|FlowControl|DoOnce false
    (:Completed
      (Default|TeleportCOOP _asbp_rowcharacter)
      (Utilities|FlowControl|Delay 0.5)
      (Default|Tplevel _asbp_rowcharacter "COOP_Lobby?listen"))))

(fn ConstructionScript
  (bind _returnvalue (Game|GetCurrentLevelName true))
  (if (Utilities|Enum|Equal(Enum) (.RightS (Utilities|String|Split _returnvalue "l" "CaseSensitive")) "10_2")
    (Variables|Default|SetLevel 10)
    (else
      (Variables|Default|SetLevel (Math|Conversions|ToInteger(Byte) (.RightS (Utilities|String|Split _returnvalue "l" "CaseSensitive")))))))