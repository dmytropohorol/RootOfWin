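; Level 1 button trigger that reacts to MainCharacter or CoolCube actors overlapping Box1.
; Each entry bumps a Human or Cube count, moves Cylinder1 to its pressed position, plays a press sound and teleports player 0, printing a debug "Hello" on success.
; Exits decrement the counts; when both reach zero, the cylinder moves back after a short delay, without rechecking occupancy.
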(event OnComponentBeginOverlap(Box1)
  (params (OverlappedComponent :type Primitive%20Component%20Object%20Reference) (OtherActor :type Actor%20Object%20Reference) (OtherComp :type Primitive%20Component%20Object%20Reference) (OtherBodyIndex :type Integer) (bFromSweep :type Boolean) (SweepResult :type Hit%20Result%20Structure%20%28by%20ref%29))
  (Utilities|Casting|CastToMainCharacter OtherActor
    (:then
      (Variables|Default|Sethuman (+ 1 (Variables|Default|Gethuman))))
    (:CastFailed
      (Utilities|Casting|CastToCoolCube OtherActor)
      (Variables|Default|Setcube (+ 1 (Variables|Default|Getcube)))))
  (Components|MoveComponentTo (Variables|Default|GetCylinder1) (Variables|Default|GetTarget%20Relative%20Location) "0, 0, 0" false false 0.2 false)
  (Audio|PlaySound2D "/Game/Audio/Button_Pressed_11.Button_Pressed_11" 1.0 1.0 0.0 0 0)
  (bind _returnvalue (Transformation|Teleport (Game|GetPlayerCharacter 0) (Variables|Default|GetDest%20Location) (Variables|Default|GetDest%20Rotation)))
  (if _returnvalue
    (Development|PrintString "Hello")))

(event OnComponentEndOverlap(Box1)
  (params (OverlappedComponent :type Primitive%20Component%20Object%20Reference) (OtherActor :type Actor%20Object%20Reference) (OtherComp :type Primitive%20Component%20Object%20Reference) (OtherBodyIndex :type Integer))
  (Utilities|Casting|CastToMainCharacter OtherActor
    (:then
      (bind _output_get (Variables|Default|Sethuman (- (Variables|Default|Gethuman) 1))))
    (:CastFailed
      (Utilities|Casting|CastToCoolCube OtherActor)
      (bind _output_get_2 (Variables|Default|Setcube (- (Variables|Default|Getcube) 1)))))
  (if (and (== _output_get_2 0) (== _output_get 0))
    (Utilities|FlowControl|Delay 1.0)
    (Components|MoveComponentTo (Variables|Default|GetCylinder1) (Variables|Default|GetTarget%20Relative%20Location_0) "0, 0, 0" false false 0.2 false)))

(fn ConstructionScript)