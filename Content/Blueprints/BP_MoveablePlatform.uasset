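; BP_MoveablePlatform is a platform actor whose Box trigger kills the player character on contact and restarts the level.
; On overlap with BP_ROWCharacter, it destroys the character, shows the W_Died widget, then reloads the current level by name after a short delay.
; The graphs contain no movement logic despite the asset's name, and Tick holds only an empty branch.
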(event OnComponentBeginOverlap(Box)
  (params (OverlappedComponent :type Primitive%20Component%20Object%20Reference) (OtherActor :type Actor%20Object%20Reference) (OtherComp :type Primitive%20Component%20Object%20Reference) (OtherBodyIndex :type Integer) (bFromSweep :type Boolean) (SweepResult :type Hit%20Result%20Structure%20%28by%20ref%29))
  (bind _asmain_character_bp (Utilities|Casting|CastToBP_ROWCharacter OtherActor))
  (Actor|DestroyActor _asmain_character_bp)
  (bind _returnvalue (UserInterface|CreateWidget "/Game/Widgets/W_Died.W_Died_C" (Game|GetPlayerController 0)))
  (UserInterface|Viewport|AddtoViewport _returnvalue 0)
  (Utilities|FlowControl|Delay 3.0)
  (bind _returnvalue_2 (Game|GetCurrentLevelName true))
  (Game|OpenLevel(byName) (Utilities|String|StringToName _returnvalue_2)))

(event EventBeginPlay)

(event Collision|EventActorBeginOverlap
  (params (OtherActor :type Actor%20Object%20Reference)))

(event EventTick
  (params (DeltaSeconds :type Float%20%28single-precision%29))
  (if true
    _))

(fn ConstructionScript)