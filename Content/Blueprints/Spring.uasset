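; Spring actor that repeatedly punches out along the X axis and eases back, as a moving launcher or obstacle.
; On BeginPlay, only the authority runs an endless latent loop that moves the root component with MoveComponentTo: a fast outward shove, a slower return, and short delays between.
; Each target is a fixed offset from the root's current world location, passed as a relative location.
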(event EventBeginPlay
  (bind _defaultsceneroot (Variables|Default|GetDefaultSceneRoot))
  (Networking|SwitchHasAuthority :!label _label
    (:Authority
      (Components|MoveComponentTo _defaultsceneroot (+ (Transformation|GetWorldLocation (Variables|Default|GetDefaultSceneRoot)) "300.000000,0.000000,0.000000") "0, 0, 0" false false 0.2 false)
      (Utilities|FlowControl|Delay 0.2)
      (Components|MoveComponentTo _defaultsceneroot (+ (Transformation|GetWorldLocation (Variables|Default|GetDefaultSceneRoot)) "-300.000000,0.000000,0.000000") "0, 0, 0" false false 2.0 false)
      (Utilities|FlowControl|Delay 1.0)
      (goto _label))))

(fn ConstructionScript)