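; BP_Button_2Level is a pressure button for level geometry, likely in the second level, that swaps hard-coded BP_Wall layouts when pressed.
; Box1 overlaps count characters and moveable cubes separately, with flags that can restrict which type presses it.
; Pressing sinks Cylinder1, plays a sound, destroys two starting walls and spawns two others.
; When both counts reach zero, a delay precedes raising the button and restoring the original walls, without rechecking the counts.
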(event OnComponentBeginOverlap(Box1)
  (params (OverlappedComponent :type Primitive%20Component%20Object%20Reference) (OtherActor :type Actor%20Object%20Reference) (OtherComp :type Primitive%20Component%20Object%20Reference) (OtherBodyIndex :type Integer) (bFromSweep :type Boolean) (SweepResult :type Hit%20Result%20Structure%20%28by%20ref%29))
  (bind _1wall (Variables|Default|Get1Wall))
  (bind _2wall (Variables|Default|Get2Wall))
  (Utilities|Casting|CastToBP_ROWCharacter OtherActor
    (:then
      (Variables|Default|SetPressedHumanCount (+ 1 (Variables|Default|GetPressedHumanCount)))
      (if (not (Variables|Default|GetisOnlyCubePressed?))
        (Components|MoveComponentTo (Variables|Default|GetCylinder1) "1.000000,1.000000,-20.161094" "0, 0, 0" false false 0.2 false :!label _label)
        (Audio|PlaySoundatLocation "/Game/Audio/Menu/Button_Pressed_11.Button_Pressed_11" (Transformation|GetWorldLocation (Variables|Default|GetBox1)) "0, 0, 0" 1.0 1.0 0.0 0 0 0 0)
        (Variables|Default|SetisPressed? true)
        (Utilities|IsValid _1wall
          (:Is%20Valid
            (Actor|DestroyActor _1wall))
          (:Is%20Not%20Valid
            _))
        (Utilities|IsValid _2wall
          (:Is%20Valid
            (Actor|DestroyActor _2wall)
            (bind _returnvalue (Game|SpawnActorfromClass "/Game/Blueprints/BP_Wall.BP_Wall_C" (Math|Transform|MakeTransform "-980.000000,1470.000000,100.000000" "0.000000,0.000000,90.000000" "1.000000,1.000000,1.000000") "Undefined" 0 0))
            (Variables|Default|Set3Wall _returnvalue)
            (bind _returnvalue_2 (Game|SpawnActorfromClass "/Game/Blueprints/BP_Wall.BP_Wall_C" (Math|Transform|MakeTransform "-580.000000,1470.000000,100.000000" "0.000000,0.000000,90.000000" "1.000000,1.000000,1.000000") "Undefined" 0 0))
            (Variables|Default|Set4Wall _returnvalue_2)))))
    (:CastFailed
      (Utilities|Casting|CastToBP_MoveableCube OtherActor)
      (Variables|Default|SetPressedCubeCount (+ 1 (Variables|Default|GetPressedCubeCount)))
      (if (not (Variables|Default|GetisOnlyHumanPressed?))
        (goto _label)))))

(event OnComponentEndOverlap(Box1)
  (params (OverlappedComponent :type Primitive%20Component%20Object%20Reference) (OtherActor :type Actor%20Object%20Reference) (OtherComp :type Primitive%20Component%20Object%20Reference) (OtherBodyIndex :type Integer))
  (bind _4wall (Variables|Default|Get4Wall))
  (bind _3wall (Variables|Default|Get3Wall))
  (Utilities|Casting|CastToBP_ROWCharacter OtherActor
    (:then
      (bind _output_get (Variables|Default|SetPressedHumanCount (- (Variables|Default|GetPressedHumanCount) 1))))
    (:CastFailed
      (Utilities|Casting|CastToBP_MoveableCube OtherActor)
      (bind _output_get_2 (Variables|Default|SetPressedCubeCount (- (Variables|Default|GetPressedCubeCount) 1)))))
  (if (and (== _output_get 0) (== _output_get_2 0))
    (Utilities|FlowControl|Delay 5.0)
    (Components|MoveComponentTo (Variables|Default|GetCylinder1) "1.000000,1.000000,-0.161094" "0, 0, 0" false false 0.2 false)
    (bind _returnvalue (Game|SpawnActorfromClass "/Game/Blueprints/BP_Wall.BP_Wall_C" (Math|Transform|MakeTransform "-780.000000,1270.000000,100.000000" "0.000000,90.000000,0.000000" "1.000000,1.000000,1.000000") "Undefined" 0 0))
    (Variables|Default|Set1Wall _returnvalue)
    (bind _returnvalue_2 (Game|SpawnActorfromClass "/Game/Blueprints/BP_Wall.BP_Wall_C" (Math|Transform|MakeTransform "-580.000000,1470.000000,100.000000" "0, 0, 0" "1.000000,1.000000,1.000000") "Undefined" 0 0))
    (Variables|Default|Set2Wall _returnvalue_2)
    (Utilities|IsValid _3wall
      (:Is%20Valid
        (Actor|DestroyActor _3wall))
      (:Is%20Not%20Valid
        _))
    (Utilities|IsValid _4wall
      (:Is%20Valid
        (Actor|DestroyActor _4wall)))))

(event EventBeginPlay
  (bind _returnvalue (Game|SpawnActorfromClass "/Game/Blueprints/BP_Wall.BP_Wall_C" (Math|Transform|MakeTransform "-780.000000,1270.000000,100.000000" "0.000000,90.000000,0.000000" "1.000000,1.000000,1.000000") "Undefined" 0 0))
  (Variables|Default|Set1Wall _returnvalue)
  (bind _returnvalue_2 (Game|SpawnActorfromClass "/Game/Blueprints/BP_Wall.BP_Wall_C" (Math|Transform|MakeTransform "-580.000000,1470.000000,100.000000" "0, 0, 0" "1.000000,1.000000,1.000000") "Undefined" 0 0))
  (Variables|Default|Set2Wall _returnvalue_2))

(fn ConstructionScript)