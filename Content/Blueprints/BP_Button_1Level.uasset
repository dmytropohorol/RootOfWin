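; Level 1 pressure button that spawns a fake wall at a fixed location on BeginPlay and destroys it when pressed.
; Box1 overlaps count MainCharacter and BP_MoveableCube occupants separately, with flags to restrict pressing to humans or cubes.
; A press lowers Cylinder1, plays a sound and sets IsPressed.
; When both counts reach zero, the button rises after ButtonDuration, but the wall stays gone.
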(event OnComponentBeginOverlap(Box1)
  (params (OverlappedComponent :type Primitive%20Component%20Object%20Reference) (OtherActor :type Actor%20Object%20Reference) (OtherComp :type Primitive%20Component%20Object%20Reference) (OtherBodyIndex :type Integer) (bFromSweep :type Boolean) (SweepResult :type Hit%20Result%20Structure%20%28by%20ref%29))
  (Utilities|Casting|CastToMainCharacter OtherActor
    (:then
      (Variables|Default|SetPressedHumanCount (+ 1 (Variables|Default|GetPressedHumanCount)))
      (if (not (Variables|Default|GetisOnlyCubePressed?))
        (Components|MoveComponentTo (Variables|Default|GetCylinder1) "1.000000,1.000000,-20.161094" "0, 0, 0" false false 0.2 false :!label _label)
        (Audio|PlaySoundatLocation "/Game/Audio/Button_Pressed_11.Button_Pressed_11" (Transformation|GetWorldLocation (Variables|Default|GetBox1)) "0, 0, 0" 1.0 1.0 0.0 0 0 0 0)
        (Variables|Default|SetisPressed? true)
        (Utilities|IsValid (stale EventBeginPlay _returnvalue)
          (:Is%20Valid
            (Actor|DestroyActor (stale EventBeginPlay _returnvalue))))))
    (:CastFailed
      (Utilities|Casting|CastToBP_MoveableCube OtherActor)
      (Variables|Default|SetPressedCubeCount (+ 1 (Variables|Default|GetPressedCubeCount)))
      (if (not (Variables|Default|GetisOnlyHumanPressed?))
        (goto _label)))))

(event OnComponentEndOverlap(Box1)
  (params (OverlappedComponent :type Primitive%20Component%20Object%20Reference) (OtherActor :type Actor%20Object%20Reference) (OtherComp :type Primitive%20Component%20Object%20Reference) (OtherBodyIndex :type Integer))
  (Utilities|Casting|CastToMainCharacter OtherActor
    (:then
      (Variables|Default|SetPressedHumanCount (- (Variables|Default|GetPressedHumanCount) 1)))
    (:CastFailed
      (Utilities|Casting|CastToBP_MoveableCube OtherActor)
      (Variables|Default|SetPressedCubeCount (- (Variables|Default|GetPressedCubeCount) 1))))
  (if (and (== (Variables|Default|GetPressedHumanCount) 0) (== (Variables|Default|GetPressedCubeCount) 0))
    (Utilities|FlowControl|Delay (Variables|Default|GetButtonDuration))
    (Components|MoveComponentTo (Variables|Default|GetCylinder1) "1.000000,1.000000,-0.161094" "0, 0, 0" false false 0.2 false)
    (Variables|Default|SetisPressed? false)))

(event EventBeginPlay
  (bind _returnvalue (Game|SpawnActorfromClass "/Game/Blueprints/BP_FakeWall.BP_FakeWall_C" (Math|Transform|MakeTransform "-180.000000,2270.000000,100.000000" "0, 0, 0" "1.000000,1.000000,1.000000") "Undefined" 0 0)))

(fn ConstructionScript)