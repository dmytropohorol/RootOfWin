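; MainGameMode is a game mode that tracks connected players, respawns their characters and handles server travel.
; PostLogin and OnLogout add and remove controllers in the AllPCs list, with removal limited to BP_ROWPlayerController.
; Respawn spawns a BP_ROWCharacter at a given transform and possesses it with the passed controller after a short delay.
; ServerTravelGM changes maps by running the ServerTravel console command with the given URL.
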(event Custom|Respawn
  (params (NewParam :type Player%20Controller%20Object%20Reference) (SpawnTransform :type Transform))
  (Utilities|IsValid NewParam
    (:Is%20Valid
      (bind _returnvalue (Game|SpawnActorfromClass "/Game/Blueprints/BP_ROWCharacter.BP_ROWCharacter_C" SpawnTransform "Undefined" "MultiplyWithRoot" 0 0))
      (Utilities|FlowControl|Delay 0.2)
      (Pawn|Possess NewParam _returnvalue))))

(event Custom|ServerTravelGM
  (params (InURL :type String))
  (Development|ExecuteConsoleCommand (Utilities|String|Append "ServerTravel " InURL) (Game|GetPlayerController 0)))

(event EventPostLogin
  (params (NewPlayer :type Player%20Controller%20Object%20Reference))
  (Utilities|Array|Add (Variables|Default|GetAll%20PCs) NewPlayer))

(event EventOnLogout
  (params (ExitingController :type Controller%20Object%20Reference))
  (bind _asbp_rowplayer_controller (Utilities|Casting|CastToBP_ROWPlayerController ExitingController))
  (Utilities|Array|RemoveItem (Variables|Default|GetAll%20PCs) _asbp_rowplayer_controller))

(fn ConstructionScript)