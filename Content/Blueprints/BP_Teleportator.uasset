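; End-of-level teleporter that records the player's progress and returns to the Menu level.
; Construction Script parses Level from the map name, treating "10_2" as 10.
; The first BP_ROWCharacter overlap async-loads "Save" for the picked slot, then rewrites that slot, incrementing its level only if it matches this one.
; It then teleports the character and writes the Level+1 achievement; Menu opens only if caching and writing succeed.
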(event OnComponentBeginOverlap(Box)
  (params (OverlappedComponent :type Primitive%20Component%20Object%20Reference) (OtherActor :type Actor%20Object%20Reference) (OtherComp :type Primitive%20Component%20Object%20Reference) (OtherBodyIndex :type Integer) (bFromSweep :type Boolean) (SweepResult :type Hit%20Result%20Structure%20%28by%20ref%29))
  (bind _returnvalue (Game|GetPlayerController 0))
  (bind _level (Variables|Default|GetLevel))
  (bind _asbp_rowcharacter (Utilities|Casting|CastToBP_ROWCharacter OtherActor))
  (Utilities|FlowControl|DoOnce false
    (:Completed
      (bind _savegame (|AsyncLoadGamefromSlot "Save")
        (:Completed
          (bind _asbp_save_game_object (Utilities|Casting|CastToBP_SaveGameObject _savegame))
          (bind _savegame_2 (|AsyncLoadGamefromSlot (Utilities|String|ToString(Integer) (Variables|/Game/Blueprints/BP_SaveGameObject.BP_SaveGameObject_C|GetSavePicked _asbp_save_game_object)))
            (:Completed
              (bind _asbp_save_game_object_2 (Utilities|Casting|CastToBP_SaveGameObject _savegame_2))
              (if (== (.level (Variables|/Game/Blueprints/BP_SaveGameObject.BP_SaveGameObject_C|GetSaveGameInformation _asbp_save_game_object_2)) _level)
                (bind _returnvalue_2 (SaveGame|CreateSaveGameObject "/Game/Blueprints/BP_SaveGameObject.BP_SaveGameObject_C"))
                (Variables|/Game/Blueprints/BP_SaveGameObject.BP_SaveGameObject_C|SetSaveGameInformation _returnvalue_2 (Utilities|Struct|MakeS_SaveGame (+ _level 1) "0001.01.01-00.00.00" (.creationtime (Variables|/Game/Blueprints/BP_SaveGameObject.BP_SaveGameObject_C|GetSaveGameInformation _asbp_save_game_object_2))))
                (|AsyncSaveGametoSlot _returnvalue_2 (Utilities|String|ToString(Integer) (Variables|/Game/Blueprints/BP_SaveGameObject.BP_SaveGameObject_C|GetSavePicked _asbp_save_game_object))
                  (:Completed
                    _))
                (else
                  (bind _returnvalue_3 (SaveGame|CreateSaveGameObject "/Game/Blueprints/BP_SaveGameObject.BP_SaveGameObject_C"))
                  (Variables|/Game/Blueprints/BP_SaveGameObject.BP_SaveGameObject_C|SetSaveGameInformation _returnvalue_3 (Utilities|Struct|MakeS_SaveGame (.level (Variables|/Game/Blueprints/BP_SaveGameObject.BP_SaveGameObject_C|GetSaveGameInformation _asbp_save_game_object_2)) "0001.01.01-00.00.00" (.creationtime (Variables|/Game/Blueprints/BP_SaveGameObject.BP_SaveGameObject_C|GetSaveGameInformation _asbp_save_game_object_2))))
                  (|AsyncSaveGametoSlot _returnvalue_3 (Utilities|String|ToString(Integer) (Variables|/Game/Blueprints/BP_SaveGameObject.BP_SaveGameObject_C|GetSavePicked _asbp_save_game_object))
                    (:Completed
                      _))))
              (Default|Teleport _asbp_rowcharacter)
              (|CacheAchievements _returnvalue
                (:OnSuccess
                  (bind _writtenachievementname (|WriteAchievementProgress _returnvalue (Utilities|String|StringToName (Utilities|String|Append "ACHIEVEMENT_" (Utilities|String|ToString(Integer) (+ (Variables|Default|GetLevel) 1)))) 1.0)
                    (:OnSuccess
                      (Development|PrintString (Utilities|String|ToString(Name) _writtenachievementname))
                      (Utilities|FlowControl|Delay 0.5)
                      (Game|OpenLevel(byName) "Menu"))))))))))))

(fn ConstructionScript
  (bind _returnvalue (Game|GetCurrentLevelName true))
  (if (Utilities|Enum|Equal(Enum) (.RightS (Utilities|String|Split _returnvalue "l" "CaseSensitive")) "10_2")
    (Variables|Default|SetLevel 10)
    (else
      (Variables|Default|SetLevel (Math|Conversions|ToInteger(Byte) (.RightS (Utilities|String|Split _returnvalue "l" "CaseSensitive")))))))