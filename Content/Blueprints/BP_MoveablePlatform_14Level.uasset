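; Moveable platform, named for level 14, whose trigger box calls Death on an overlapping BP_ROWCharacter or BP_Cube9level.
; MoveCube alternately plays and reverses a Timeline that drives the Cube's relative location through a FlipFlop.
; Cube materials swap between two variants per Team symbol during movement and on finish, using direction-gated DoOnce nodes and a flag.
; The construction script sets the initial variant from Team and THXUE5; both character overlap functions are empty.
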(event OnComponentBeginOverlap(Box)
  (params (OverlappedComponent :type Primitive%20Component%20Object%20Reference) (OtherActor :type Actor%20Object%20Reference) (OtherComp :type Primitive%20Component%20Object%20Reference) (OtherBodyIndex :type Integer) (bFromSweep :type Boolean) (SweepResult :type Hit%20Result%20Structure%20%28by%20ref%29))
  (bind _asbp_rowcharacter (Utilities|Casting|CastToBP_ROWCharacter OtherActor)
    (:then
      (Default|Death _asbp_rowcharacter))
    (:CastFailed
      (bind _asbp_cube_9level (Utilities|Casting|CastToBP_Cube9level OtherActor))
      (Default|Death _asbp_cube_9level))))

(event Custom|MoveCube
  (bind _cube (Variables|Default|GetCube))
  (bind _cube_2 (Variables|Default|GetCube))
  (bind _cube_3 (Variables|Default|GetCube))
  (bind _cube_4 (Variables|Default|GetCube))
  (Utilities|FlowControl|FlipFlop
    (:A
      (bind (_direction _newtrack_0) (Timeline|Timeline Play)
        (:Update
          (Transformation|SetRelativeLocation (Variables|Default|GetCube) _newtrack_0 false false)
          (switch Utilities|FlowControl|Switch|SwitchonETimelineDirection _direction
            (:Forward
              (Utilities|FlowControl|DoOnce false :!label _label
                (:Completed
                  (Utilities|FlowControl|Sequence
                    (:then_0
                      (goto _label_2 Reset))
                    (:then_1
                      (Variables|Default|SetNewVar true)
                      (switch Utilities|FlowControl|Switch|SwitchonL14_MoveableCubesTeams (Variables|Default|GetTeam)
                        (:NewEnumerator0
                          (Rendering|Material|SetMaterial _cube_2 0 "/Game/Materials/Teams/M_CubeTeam2.M_CubeTeam2"))
                        (:NewEnumerator1
                          (Rendering|Material|SetMaterial _cube_2 0 "/Game/Materials/Teams/M_StarTeam1.M_StarTeam1"))
                        (:NewEnumerator2
                          (Rendering|Material|SetMaterial _cube_2 0 "/Game/Materials/Teams/M_CubeWithoutTeam1.M_CubeWithoutTeam1"))
                        (:NewEnumerator3
                          (Rendering|Material|SetMaterial _cube_2 0 "/Game/Materials/Teams/M_CircleTeam1.M_CircleTeam1"))
                        (:NewEnumerator4
                          (Rendering|Material|SetMaterial _cube_2 0 "/Game/Materials/Teams/M_6xTeam2.M_6xTeam2"))))))))
            (:Backward
              (Utilities|FlowControl|DoOnce false :!label _label_2
                (:Completed
                  (Utilities|FlowControl|Sequence
                    (:then_0
                      (goto _label Reset))
                    (:then_1
                      (Variables|Default|SetNewVar false)
                      (switch Utilities|FlowControl|Switch|SwitchonL14_MoveableCubesTeams (Variables|Default|GetTeam)
                        (:NewEnumerator0
                          (Rendering|Material|SetMaterial _cube 0 "/Game/Materials/Teams/M_CubeTeam1.M_CubeTeam1"))
                        (:NewEnumerator1
                          (Rendering|Material|SetMaterial _cube 0 "/Game/Materials/Teams/M_StarTeam2.M_StarTeam2"))
                        (:NewEnumerator2
                          (Rendering|Material|SetMaterial _cube 0 "/Game/Materials/Teams/M_CubeWithoutTeam2.M_CubeWithoutTeam2"))
                        (:NewEnumerator3
                          (Rendering|Material|SetMaterial _cube 0 "/Game/Materials/Teams/M_CircleTeam2.M_CircleTeam2"))
                        (:NewEnumerator4
                          (Rendering|Material|SetMaterial _cube 0 "/Game/Materials/Teams/M_6xTeam1.M_6xTeam1"))))))))))
        (:Finished
          (if (Variables|Default|GetNewVar)
            (switch Utilities|FlowControl|Switch|SwitchonL14_MoveableCubesTeams (Variables|Default|GetTeam)
              (:NewEnumerator0
                (Rendering|Material|SetMaterial _cube_4 0 "/Game/Materials/Teams/M_CubeTeam1.M_CubeTeam1"))
              (:NewEnumerator1
                (Rendering|Material|SetMaterial _cube_4 0 "/Game/Materials/Teams/M_StarTeam2.M_StarTeam2"))
              (:NewEnumerator2
                (Rendering|Material|SetMaterial _cube_4 0 "/Game/Materials/Teams/M_CubeWithoutTeam2.M_CubeWithoutTeam2"))
              (:NewEnumerator3
                (Rendering|Material|SetMaterial _cube_4 0 "/Game/Materials/Teams/M_CircleTeam2.M_CircleTeam2"))
              (:NewEnumerator4
                (Rendering|Material|SetMaterial _cube_4 0 "/Game/Materials/Teams/M_6xTeam1.M_6xTeam1")))
            (else
              (switch Utilities|FlowControl|Switch|SwitchonL14_MoveableCubesTeams (Variables|Default|GetTeam)
                (:NewEnumerator0
                  (Rendering|Material|SetMaterial _cube_3 0 "/Game/Materials/Teams/M_CubeTeam2.M_CubeTeam2"))
                (:NewEnumerator1
                  (Rendering|Material|SetMaterial _cube_3 0 "/Game/Materials/Teams/M_StarTeam1.M_StarTeam1"))
                (:NewEnumerator2
                  (Rendering|Material|SetMaterial _cube_3 0 "/Game/Materials/Teams/M_CubeWithoutTeam1.M_CubeWithoutTeam1"))
                (:NewEnumerator3
                  (Rendering|Material|SetMaterial _cube_3 0 "/Game/Materials/Teams/M_CircleTeam1.M_CircleTeam1"))
                (:NewEnumerator4
                  (Rendering|Material|SetMaterial _cube_3 0 "/Game/Materials/Teams/M_6xTeam2.M_6xTeam2"))))))))
    (:B
      (Timeline|Timeline Reverse))))

(fn ConstructionScript
  (bind _cube (Variables|Default|GetCube))
  (switch Utilities|FlowControl|Switch|SwitchonL14_MoveableCubesTeams (Variables|Default|GetTeam)
    (:NewEnumerator0
      (if (Variables|Default|GetTHXUE5)
        (Rendering|Material|SetMaterial _cube 0 "/Game/Materials/Teams/M_CubeTeam2.M_CubeTeam2")
        (else
          (Rendering|Material|SetMaterial _cube 0 "/Game/Materials/Teams/M_CubeTeam1.M_CubeTeam1"))))
    (:NewEnumerator1
      (if (Variables|Default|GetTHXUE5)
        (Rendering|Material|SetMaterial _cube 0 "/Game/Materials/Teams/M_StarTeam2.M_StarTeam2")
        (else
          (Rendering|Material|SetMaterial _cube 0 "/Game/Materials/Teams/M_StarTeam1.M_StarTeam1"))))
    (:NewEnumerator2
      (if (Variables|Default|GetTHXUE5)
        (Rendering|Material|SetMaterial _cube 0 "/Game/Materials/Teams/M_CubeWithoutTeam2.M_CubeWithoutTeam2")
        (else
          (Rendering|Material|SetMaterial _cube 0 "/Game/Materials/Teams/M_CubeWithoutTeam1.M_CubeWithoutTeam1"))))
    (:NewEnumerator3
      (if (Variables|Default|GetTHXUE5)
        (Rendering|Material|SetMaterial _cube 0 "/Game/Materials/Teams/M_CircleTeam2.M_CircleTeam2")
        (else
          (Rendering|Material|SetMaterial _cube 0 "/Game/Materials/Teams/M_CircleTeam1.M_CircleTeam1"))))
    (:NewEnumerator4
      (if (Variables|Default|GetTHXUE5)
        (Rendering|Material|SetMaterial _cube 0 "/Game/Materials/Teams/M_6xTeam2.M_6xTeam2")
        (else
          (Rendering|Material|SetMaterial _cube 0 "/Game/Materials/Teams/M_6xTeam1.M_6xTeam1"))))))

(fn CharacterEndOverlap
  (params (NewParam :type Boolean))
  (return))

(fn CharacterStartOverlap
  (params (NewParam :type Boolean))
  (return))