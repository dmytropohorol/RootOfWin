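; BP_Mark is a marker actor that displays its distance to the player through a widget component.
; On BeginPlay it passes a fixed reddish color to the widget.
; Every tick it measures the distance to player character 0, converts it to truncated whole meters, and pushes that number with a "meters" suffix to the widget as text.
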(event EventBeginPlay
  (Class|BPIMarker|UpdateColor(Message) (UserInterface|GetUserWidgetObject (Variables|Default|GetWidget)) "(R=1.000000,G=0.166081,B=0.195929,A=1.000000)"))

(event EventTick
  (params (DeltaSeconds :type Float%20%28single-precision%29))
  (Class|BPIMarker|UpdateText(Message) (UserInterface|GetUserWidgetObject (Variables|Default|GetWidget)) (Utilities|Text|ToText(String) (Utilities|String|Append (Utilities|String|ToString(Integer) (Math|Float|Truncate (/ (Math|Vector|Distance(Vector) (Transformation|GetActorLocation) (Transformation|GetActorLocation (Game|GetPlayerCharacter 0))) 1e+02))) " meters"))))

(fn ConstructionScript)