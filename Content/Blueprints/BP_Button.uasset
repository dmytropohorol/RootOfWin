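; BP_Button is a pressure button that characters and cubes press by overlapping its Box1 trigger.
; Separate human and cube counters track occupants, while human-only and cube-only flags filter what triggers a press.
; A press lowers the cylinder, plays a sound and sets IsPressed; once both counts reach zero, it rises after ButtonDuration.
; An actor-spawning chain with optional delayed repeat exists but is never run.
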(event OnComponentBeginOverlap(Box1)
  (params (OverlappedComponent :type Primitive%20Component%20Object%20Reference) (OtherActor :type Actor%20Object%20Reference) (OtherComp :type Primitive%20Component%20Object%20Reference) (OtherBodyIndex :type Integer) (bFromSweep :type Boolean) (SweepResult :type Hit%20Result%20Structure%20%28by%20ref%29))
  (Utilities|Casting|CastToBP_ROWCharacter OtherActor
    (:then
      (Variables|Default|SetPressedHumanCount (+ 1 (Variables|Default|GetPressedHumanCount)))
      (if (not (Variables|Default|GetisOnlyCubePressed?))
        (Components|MoveComponentTo (Variables|Default|GetCylinder1) "1.000000,1.000000,0.418798" "0, 0, 0" false false 0.2 false :!label _label)
        (Audio|PlaySoundatLocation "/Game/Audio/Menu/Button_Pressed_11.Button_Pressed_11" (Transformation|GetWorldLocation (Variables|Default|GetBox1)) "0, 0, 0" 1.0 1.0 0.0 0 0 0 0)
        (Variables|Default|SetisPressed? true)))
    (:CastFailed
      (Utilities|Casting|CastToBP_Cube OtherActor)
      (Variables|Default|SetPressedCubeCount (+ 1 (Variables|Default|GetPressedCubeCount)))
      (if (not (Variables|Default|GetisOnlyHumanPressed?))
        (goto _label)))))

(event OnComponentEndOverlap(Box1)
  (params (OverlappedComponent :type Primitive%20Component%20Object%20Reference) (OtherActor :type Actor%20Object%20Reference) (OtherComp :type Primitive%20Component%20Object%20Reference) (OtherBodyIndex :type Integer))
  (Utilities|Casting|CastToBP_ROWCharacter OtherActor
    (:then
      (Variables|Default|SetPressedHumanCount (- (Variables|Default|GetPressedHumanCount) 1)))
    (:CastFailed
      (Utilities|Casting|CastToBP_Cube OtherActor)
      (Variables|Default|SetPressedCubeCount (- (Variables|Default|GetPressedCubeCount) 1))))
  (if (and (== (Variables|Default|GetPressedHumanCount) 0) (== (Variables|Default|GetPressedCubeCount) 0))
    (Utilities|FlowControl|Delay (Variables|Default|GetButtonDuration))
    (Components|MoveComponentTo (Variables|Default|GetCylinder1) "1.000000,1.000000,8.670346" "0, 0, 0" false false 0.2 false)
    (Audio|PlaySoundatLocation "/Game/Audio/Menu/Button_Pressed_11.Button_Pressed_11" (Transformation|GetWorldLocation (Variables|Default|GetBox1)) "0, 0, 0" 1.0 1.0 0.0 0 0 0 0)
    (Variables|Default|SetisPressed? false)))

(fn ConstructionScript)